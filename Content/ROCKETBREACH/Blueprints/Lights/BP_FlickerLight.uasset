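; BP_FlickerLight is a light actor whose rect light flickers randomly during play.
; On BeginPlay a self-calling event randomly sets the light to zero or its base intensity, weighted toward base intensity, then waits a random delay within a min/max range before repeating.
; When flickering is disabled, the event sets the light to base intensity and the loop stops.
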(event Custom|FlickerLight
  (if (Variables|Default|GetFlickerEnabled)
    (Rendering|Components|Light|SetIntensity (Variables|Default|GetRectLight) (Math|Float|SelectFloat 0.0 (Variables|Default|GetBaseIntensity) (Math|Random|RandomBoolwithWeight 0.25)))
    (Utilities|FlowControl|Delay (Math|Random|RandomFloatinRange (Variables|Default|GetFlickerSpeedMin) (Variables|Default|GetFlickerSpeedMax)))
    (CallFunction|FlickerLight)
    (else
      (Rendering|Components|Light|SetIntensity (Variables|Default|GetRectLight) (Variables|Default|GetBaseIntensity)))))

(event EventBeginPlay
  (CallFunction|FlickerLight))

(event Collision|EventActorBeginOverlap
  (params (OtherActor :type Actor%20Object%20Reference)))

(event EventTick
  (params (DeltaSeconds :type Float%20%28single-precision%29)))

(fn ConstructionScript)