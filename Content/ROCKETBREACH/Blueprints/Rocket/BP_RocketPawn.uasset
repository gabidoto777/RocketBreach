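; BP_RocketPawn is a player-controlled rocket pawn flown through physics thrust.
; Space and WASD set boolean flags for main thrust and four rotation directions while held.
; Each Tick, active flags push PhysicsBody along their thrust point's up vector at that point's location, so off-center side thrusters can rotate it.
; A descent assist branch exists but does nothing, and its gravity-compensation math is unused.
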(event EventTick
  (params (DeltaSeconds :type Float%20%28single-precision%29))
  (Utilities|FlowControl|Sequence
    (:then_0
      (if (Variables|Default|GetThrusting)
        (Class|PrimitiveComponent|AddForceatLocation (Variables|Default|GetPhysicsBody) (* (Math|Vector|GetUpVector (Variables|Default|GetMainThrustPoint)) (Variables|RocketMovement|GetMainThrustForce)) (Transformation|GetWorldLocation (Variables|Default|GetMainThrustPoint)) "None")))
    (:then_1
      (if (Variables|Default|GetRotatingWest)
        (Class|PrimitiveComponent|AddForceatLocation (Variables|Default|GetPhysicsBody) (* (Math|Vector|GetUpVector (Variables|Default|GetLeftThrustPoint)) (Variables|RocketMovement|GetSideThrustForce)) (Transformation|GetWorldLocation (Variables|Default|GetLeftThrustPoint)) "None")))
    (:then_2
      (if (Variables|Default|GetRotatingEast)
        (Class|PrimitiveComponent|AddForceatLocation (Variables|Default|GetPhysicsBody) (* (Math|Vector|GetUpVector (Variables|Default|GetRightThrustPoint)) (Variables|RocketMovement|GetSideThrustForce)) (Transformation|GetWorldLocation (Variables|Default|GetRightThrustPoint)) "None")))
    (:then_3
      (if (Variables|Default|GetRotatingNorth)
        (Class|PrimitiveComponent|AddForceatLocation (Variables|Default|GetPhysicsBody) (* (Math|Vector|GetUpVector (Variables|Default|GetNorthThrustPoint)) (Variables|RocketMovement|GetSideThrustForce)) (Transformation|GetWorldLocation (Variables|Default|GetNorthThrustPoint)) "None")))
    (:then_4
      (if (Variables|Default|GetRotatingSouth)
        (Class|PrimitiveComponent|AddForceatLocation (Variables|Default|GetPhysicsBody) (* (Math|Vector|GetUpVector (Variables|Default|GetSouthThrustPoint)) (Variables|RocketMovement|GetSideThrustForce)) (Transformation|GetWorldLocation (Variables|Default|GetSouthThrustPoint)) "None")))
    (:then_5
      (if (Variables|Default|GetDescentAssistEnabled)
        _))))

(event Input|KeyboardEvents|S
  (params (Key :type Key%20Structure :default "None"))
  (:Pressed
    (Variables|Default|SetRotatingSouth true))
  (:Released
    (Variables|Default|SetRotatingSouth false)))

(event Input|KeyboardEvents|SpaceBar
  (params (Key :type Key%20Structure :default "None"))
  (:Pressed
    (Variables|Default|SetThrusting true))
  (:Released
    (Variables|Default|SetThrusting false)))

(event Input|KeyboardEvents|A
  (params (Key :type Key%20Structure :default "None"))
  (:Pressed
    (Variables|Default|SetRotatingWest true))
  (:Released
    (Variables|Default|SetRotatingWest false)))

(event Input|KeyboardEvents|D
  (params (Key :type Key%20Structure :default "None"))
  (:Pressed
    (Variables|Default|SetRotatingEast true))
  (:Released
    (Variables|Default|SetRotatingEast false)))

(event Input|KeyboardEvents|W
  (params (Key :type Key%20Structure :default "None"))
  (:Pressed
    (Variables|Default|SetRotatingNorth true))
  (:Released
    (Variables|Default|SetRotatingNorth false)))

(fn ConstructionScript)